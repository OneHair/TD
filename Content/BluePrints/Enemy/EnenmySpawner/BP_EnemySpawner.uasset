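; BP_EnemySpawner spawns a given array of enemy classes one after another at its EnemySpawnPos transform.
; SpawnEnemyArray stores the array and passes its length to Spawn, which always spawns regardless of collision.
; Spawn loops by calling itself after a GapTime delay, advancing a member index and resetting it once the array is done.
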(event `SpawnEnemyArray`
  (params (EnenmyArray :type "Array of /Game/BluePrints/Enemy/BP_EnemyBase Class Reference"))
  (bind _output_get (set `self.EnemyArrayTemp` EnenmyArray))
  (`self.Spawn` (`KismetArrayLibrary.Array_Length` _output_get)))

(event `Spawn`
  (params (CycleTime :type Integer))
  (if (<= (`self.CycleTimeTemp`) (- CycleTime 1))
    (`|SpawnActorFromClass` (`|GetArrayItem` (`self.EnemyArrayTemp`) (`self.CycleTimeTemp`)) (`SceneComponent.K2_GetComponentToWorld` (`self.EnemySpawnPos`)) "AlwaysSpawn" "OverrideRootScale" null null)
    (`KismetSystemLibrary.Delay` (`self.GapTime`))
    (`/Engine/EditorBlueprintResources/StandardMacros.IncrementInt` (`self.CycleTimeTemp`)
      (:`  `
        (`self.Spawn` CycleTime)))
    (else
      (set `self.CycleTimeTemp` 0))))

(fn `UserConstructionScript`)