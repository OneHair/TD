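; BP_EnemyBase is a tower defense enemy that moves toward the BP_CoreTower at its configured speed.
; Tick looks up the core tower and reissues AIMoveTo every frame, with only a debug print on arrival.
; GetDamage lowers clamped HP and calls Die at zero.
; Die deals burst damage with linear distance falloff to every BP_TowerBase, destroys the actor and adds Bonus to the player camera's LeftMoney.
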(event `self.ReceiveBeginPlay`
  (set `CharacterMovementComponent.MaxWalkSpeed` (`self.Speed`) (`self.CharacterMovement`)))

(event `self.ReceiveTick`
  (params (DeltaSeconds :type "Float (single-precision)"))
  (bind _outactors (`GameplayStatics.GetAllActorsOfClass` "/Game/BluePrints/Tower/BP_CoreTower.BP_CoreTower_C"))
  (bind _output (`|GetArrayItem` _outactors))
  (`/Engine/EditorBlueprintResources/StandardMacros.IsValid` _output
    (:`Is Valid`
      (`|AIMoveTo` self (0.0 0.0 0.0) _output
        (:`OnSuccess`
          (`KismetSystemLibrary.PrintString` "Hello"))))))

(event `GetDamage`
  (params (Damage :type Integer))
  (bind _output_get (set `self.HP` (`KismetMathLibrary.Clamp` (- (`self.HP`) Damage) 0 100)))
  (if (<= _output_get 0)
    (`self.Die`)))

(event `Die`
  (bind _burstrange (`self.BurstRange`))
  (bind _playercamera (`/Game/BluePrints/GamePlay/BP_TDPlayercontroller.PlayerCamera` (cast `/Game/BluePrints/GamePlay/BP_TDPlayercontroller` (`GameplayStatics.GetPlayerController` 0) :!pure true)))
  (`KismetSystemLibrary.PrintString` "Die!!!!")
  (bind _outactors (`GameplayStatics.GetAllActorsOfClass` "/Game/BluePrints/Tower/BP_TowerBase.BP_TowerBase_C"))
  (for _array_element _outactors
    (`/Game/BluePrints/Tower/BP_TowerBase.GetDamage` _array_element (* (/ (`KismetMathLibrary.FClamp` (- _burstrange (`KismetMathLibrary.VSize` (- (`self.K2_GetActorLocation` _array_element) (`self.K2_GetActorLocation`)))) 0.0 _burstrange) (`self.BurstRange`)) (`self.BurstDamage`))))
  (`self.K2_DestroyActor`)
  (set `/Game/BluePrints/GamePlay/BP_CameraPawn.LeftMoney` (+ (`self.Bonus`) (`/Game/BluePrints/GamePlay/BP_CameraPawn.LeftMoney` _playercamera)) _playercamera))

(fn `UserConstructionScript`)