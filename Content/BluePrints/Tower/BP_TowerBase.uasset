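; BP_TowerBase is the base tower defense tower, snapped to a TileManager tile and registered there on construction.
; It tracks BP_EnemyBase actors in AttackRange, aims FirePos at the first and spawns targeted bullets on a reload delay.
; A directional line trace links it to a source tower, deriving its energy from that tower and ModifyEnergy.
; Damage destroys it, while clicking opens a modify widget and recyclable towers refund their cost on removal.
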(event `self.ReceiveTick`
  (params (DeltaSeconds :type "Float (single-precision)"))
  (bind _firepos (`self.FirePos`))
  (bind _output (`|GetArrayItem` (`self.EnenmyInRange`)))
  ;[1 1 1] Tick
  (`/Engine/EditorBlueprintResources/StandardMacros.IsValid` _output
    (:`Is Valid`
      (`SceneComponent.K2_SetWorldRotation` _firepos (`KismetMathLibrary.FindLookAtRotation` (`SceneComponent.K2_GetComponentLocation` _firepos) (`self.K2_GetActorLocation` _output)) false false)
      (`self.Shot` _output))))

(event `GetDamage`
  (params (Damage :type "Float (double-precision)"))
  ;[1 1 1] GetDamage
  (bind _output_get (set `self.HP` (- (`self.HP`) Damage)))
  (if (<= _output_get 0.0)
    (`self.K2_DestroyActor`)))

(event `Shot`
  (params (TargetEnemy :type "/Game/BluePrints/Enemy/BP_EnemyBase Object Reference"))
  (bind _firepos (`self.FirePos`))
  ;[1 1 1] Shot
  (if (`self.CanFire?`)
    (set `self.CanFire?` false)
    (bind _returnvalue (`|SpawnActorFromClass` (`self.BulletClass`) (`KismetMathLibrary.MakeTransform` (`SceneComponent.K2_GetComponentLocation` _firepos) (`SceneComponent.K2_GetComponentRotation` _firepos)) "Undefined" "OverrideRootScale" null null))
    (set `/Game/BluePrints/Tower/Bullets/BP_BulletBase.TargetEnemy` TargetEnemy _returnvalue)
    (`KismetSystemLibrary.Delay` (`self.ReloadTime`))
    (set `self.CanFire?` true)))

(event `self.AttackRange.OnComponentEndOverlap`
  (params (OverlappedComponent :type "PrimitiveComponent Object Reference") (OtherActor :type "Actor Object Reference") (OtherComp :type "PrimitiveComponent Object Reference") (OtherBodyIndex :type Integer))
  ;[1 1 1] UpdateEnenmyArray
  (bind _asbp_enemy_base (cast `/Game/BluePrints/Enemy/BP_EnemyBase` OtherActor))
  (`KismetArrayLibrary.Array_RemoveItem` (`self.EnenmyInRange`) _asbp_enemy_base))

(event `self.AttackRange.OnComponentBeginOverlap`
  (params (OverlappedComponent :type "PrimitiveComponent Object Reference") (OtherActor :type "Actor Object Reference") (OtherComp :type "PrimitiveComponent Object Reference") (OtherBodyIndex :type Integer) (bFromSweep :type Boolean) (SweepResult :type "HitResult Structure (by ref)"))
  ;[1 1 1] UpdateEnenmyArray
  (bind _asbp_enemy_base (cast `/Game/BluePrints/Enemy/BP_EnemyBase` OtherActor))
  (`KismetArrayLibrary.Array_AddUnique` (`self.EnenmyInRange`) _asbp_enemy_base))

(event `ChangeEnergyFrom`
  (params (Where :type "/Game/BluePrints/Tower/Energy/EnergySource Enum" :default "NewEnumerator0"))
  (bind (_energyleft _attributekind _attackkind) (break `/Game/BluePrints/Tower/Energy/EnergyNova` (`self.ModifyEnergy`)))
  (bind _returnvalue (+ (`self.K2_GetActorLocation`) (0.0 0.0 200.0)))
  ;[1 1 1] ChangeEnergy
  (switch `/Game/BluePrints/Tower/Energy/EnergySource` Where
    (:`NewEnumerator0`
      (set `self.TempTargetVector` (10000.0 0.0 0.0)))
    (:`NewEnumerator1`
      (set `self.TempTargetVector` (-10000.0 0.0 0.0)))
    (:`NewEnumerator2`
      (set `self.TempTargetVector` (0.0 -10000.0 0.0)))
    (:`NewEnumerator3`
      (set `self.TempTargetVector` (0.0 10000.0 0.0))))
  (bind _outhit (`KismetSystemLibrary.LineTraceSingle` :`Start` _returnvalue :`End` (+ _returnvalue (`self.TempTargetVector`)) :`TraceChannel` "TraceTypeQuery1" :`DrawDebugType` "ForDuration"))
  (bind _asbp_tower_base (cast `/Game/BluePrints/Tower/BP_TowerBase` (`.HitActor` (`GameplayStatics.BreakHitResult` _outhit))))
  (set `self.EnergySourceTower` _asbp_tower_base)
  (bind _output_get (set `self.CurrentEnergy` (make `/Game/BluePrints/Tower/Energy/EnergyNova` (- (`.EnergyLeft_3_08BADB0A4886F5B9E6559D905F9881EA` (break `/Game/BluePrints/Tower/Energy/EnergyNova` (`/Game/BluePrints/Tower/BP_TowerBase.CurrentEnergy` (`self.EnergySourceTower`)))) _energyleft) _attributekind _attackkind)))
  (bind (_energyleft_2 _attributekind_2 _attackkind_2) (break `/Game/BluePrints/Tower/Energy/EnergyNova` _output_get))
  ;;[1 1 1] Test
  (`KismetSystemLibrary.PrintString` (`KismetStringLibrary.Conv_IntToString` _energyleft_2))
  (`KismetSystemLibrary.PrintString` (`|GetEnumeratorNameAsString` _attributekind_2))
  (`KismetSystemLibrary.PrintString` (`|GetEnumeratorNameAsString` _attackkind_2)))

(event `self.ReceiveActorOnClicked`
  (params (ButtonPressed :type "Key Structure"))
  ;[1 1 1] BeChoosed
  (if (not (`/Game/BluePrints/GamePlay/BP_TDPlayercontroller.ReadyToConfirm` (cast `/Game/BluePrints/GamePlay/BP_TDPlayercontroller` (`GameplayStatics.GetPlayerController` 0) :!pure true)))
    (bind _returnvalue (`|CreateWidget` "/Game/UMG/ModifyTower.ModifyTower_C" null self))
    (`UserWidget.AddToViewport` _returnvalue 0)))

(event `RemoveFromMap`
  (bind _playercamera (`/Game/BluePrints/GamePlay/BP_TDPlayercontroller.PlayerCamera` (cast `/Game/BluePrints/GamePlay/BP_TDPlayercontroller` (`GameplayStatics.GetPlayerController` 0) :!pure true)))
  ;[1 1 1] Remove
  (if (`self.CanBeRecycle?`)
    (set `/Game/BluePrints/GamePlay/BP_CameraPawn.LeftMoney` (+ (`self.Cost`) (`/Game/BluePrints/GamePlay/BP_CameraPawn.LeftMoney` _playercamera)) _playercamera)
    (`Widget.RemoveFromParent` (stale `self.ReceiveActorOnClicked` _returnvalue))
    (`self.K2_DestroyActor`)
    (else
      (`KismetSystemLibrary.PrintString` "This tower cannot be recycle"))))

(fn `UserConstructionScript`
  (bind _tilemanager (`self.TileManager`))
  (`/Engine/EditorBlueprintResources/StandardMacros.IsValid` _tilemanager
    (:`Is Valid`
      (bind _instancetransform (`/Game/BluePrints/GamePlay/TileManager.GetInstanceTransform` _tilemanager (`self.K2_GetActorLocation`)))
      (`SceneComponent.K2_SetWorldLocation` (`self.StaticMesh`) (`KismetMathLibrary.MakeVector` (.x (.location _instancetransform)) (.y (.location _instancetransform)) (+ (.z (.location _instancetransform)) 200.0)) false false)
      (`KismetArrayLibrary.Array_AddUnique` (`/Game/BluePrints/GamePlay/TileManager.TowerArray` _tilemanager) self))))