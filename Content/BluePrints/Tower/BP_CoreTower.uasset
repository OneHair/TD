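; BP_CoreTower is the core tower, whose loss of all HP means the player loses.
; CoreGetDamage subtracts Damage from HP, or prints a lose message without updating HP when the hit would bring it to zero or below.
; The DamageRange overlap only casts the other actor to BP_EnemyBase, with nothing wired after it, so it deals no damage here.
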(event `self.DamageRange.OnComponentBeginOverlap`
  (params (OverlappedComponent :type "PrimitiveComponent Object Reference") (OtherActor :type "Actor Object Reference") (OtherComp :type "PrimitiveComponent Object Reference") (OtherBodyIndex :type Integer) (bFromSweep :type Boolean) (SweepResult :type "HitResult Structure (by ref)"))
  (cast `/Game/BluePrints/Enemy/BP_EnemyBase` OtherActor))

(event `CoreGetDamage`
  (bind _returnvalue (- (`self.HP`) (`self.Damage`)))
  (if (<= _returnvalue 0.0)
    (`KismetSystemLibrary.PrintString` "YOU LOSE!!!!!!!!!")
    (else
      (set `self.HP` _returnvalue))))

(fn `UserConstructionScript`
  (`parent.UserConstructionScript`))