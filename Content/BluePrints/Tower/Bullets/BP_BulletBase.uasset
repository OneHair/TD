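; BP_BulletBase is the base tower projectile that homes in on a target enemy.
; Each tick it turns toward the target's location and moves along its sphere's forward vector by BulletSpeed, destroying itself if the target becomes invalid.
; When the sphere begins overlapping any BP_EnemyBase, it applies Damage through GetDamage and destroys itself.
; Movement is a per-tick world offset without sweep or delta-time scaling, so speed depends on frame rate.
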(event `self.ReceiveTick`
  (params (DeltaSeconds :type "Float (single-precision)"))
  (bind _targetenemy (`self.TargetEnemy`))
  (`/Engine/EditorBlueprintResources/StandardMacros.IsValid` _targetenemy
    (:`Is Valid`
      (`self.K2_SetActorRotation` self (`KismetMathLibrary.FindLookAtRotation` (`self.K2_GetActorLocation` self) (`self.K2_GetActorLocation` _targetenemy)) false)
      (`self.K2_AddActorWorldOffset` (* (`SceneComponent.GetForwardVector` (`self.Sphere`)) (`self.BulletSpeed`))))
    (:`Is Not Valid`
      (`self.K2_DestroyActor`))))

(event `self.Sphere.OnComponentBeginOverlap`
  (params (OverlappedComponent :type "PrimitiveComponent Object Reference") (OtherActor :type "Actor Object Reference") (OtherComp :type "PrimitiveComponent Object Reference") (OtherBodyIndex :type Integer) (bFromSweep :type Boolean) (SweepResult :type "HitResult Structure (by ref)"))
  (bind _asbp_enemy_base (cast `/Game/BluePrints/Enemy/BP_EnemyBase` OtherActor))
  (`/Game/BluePrints/Enemy/BP_EnemyBase.GetDamage` _asbp_enemy_base (`self.Damage`))
  (`self.K2_DestroyActor`))

(fn `UserConstructionScript`)