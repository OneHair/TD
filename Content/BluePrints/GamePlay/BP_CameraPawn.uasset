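; Player camera pawn for a tower defense game that handles view movement and tower placement.
; Axis inputs pan it horizontally, while the zoom actions tilt its pitch, which is clamped every Tick.
; Each Tick also traces under the mouse to move the pending tower, snapping it atop TileManager instances.
; Confirm passes that tower, tile and snapped location to BP_TDPlayercontroller to build.
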(event `InputAxis|MoveForward`
  (params (AxisValue :type "Float (single-precision)"))
  (bind (_returnvalue_x _returnvalue_y) (`KismetMathLibrary.BreakVector` (`SceneComponent.GetForwardVector` (`self.DefaultSceneRoot`))))
  ;[1 1 1] CameraControl
  (`self.K2_AddActorWorldOffset` (* (* (`KismetMathLibrary.MakeVector` _returnvalue_x _returnvalue_y) (`self.Speed`)) AxisValue)))

(event `InputAxis|MoveRight`
  (params (AxisValue :type "Float (single-precision)"))
  (bind (_returnvalue_x _returnvalue_y) (`KismetMathLibrary.BreakVector` (`SceneComponent.GetRightVector` (`self.DefaultSceneRoot`))))
  ;[1 1 1] CameraControl
  (`self.K2_AddActorWorldOffset` (* (* (`KismetMathLibrary.MakeVector` _returnvalue_x _returnvalue_y) (`self.Speed`)) AxisValue)))

(event `InputAction|ZoomUP`
  (params (Key :type "Key Structure"))
  ;[1 1 1] CameraControl
  (:`Pressed`
    (`self.K2_AddActorWorldRotation` self (`KismetMathLibrary.MakeRotator` 0.0 (* (`self.RotateSpeed`) -1.0)) false false)))

(event `self.ReceiveTick`
  (params (DeltaSeconds :type "Float (single-precision)"))
  (bind (_returnvalue_roll _returnvalue_pitch _returnvalue_yaw) (`KismetMathLibrary.BreakRotator` (`self.K2_GetActorRotation`)))
  (bind _presenttower (`self.PresentTower`))
  (bind (_worldlocation _worlddirection) (`PlayerController.DeprojectMousePositionToWorld` (`GameplayStatics.GetPlayerController` 0)))
  (`|ExecutionSequence`
    (:`then_0`
      (`/Engine/EditorBlueprintResources/StandardMacros.IsValid` _presenttower
        (:`Is Valid`
          (`KismetArrayLibrary.Array_AddUnique` (`self.ActorToIgnore`) _presenttower)
          (bind _outhit (`KismetSystemLibrary.LineTraceSingle` _worldlocation (+ _worldlocation (* _worlddirection 10000.0)) "TraceTypeQuery1" false (`self.ActorToIgnore`) "ForOneFrame"))
          (set `self.HitInfo` _outhit)
          (bind (_bblockinghit _binitialoverlap _time _distance _location _impactpoint _normal _impactnormal _physmat _hitactor) (`GameplayStatics.BreakHitResult` _outhit))
          (bind _astile_manager (cast `/Game/BluePrints/GamePlay/TileManager` _hitactor)
            (:`then`
              (bind _instancetransform (`/Game/BluePrints/GamePlay/TileManager.GetInstanceTransform` _astile_manager _location))
              (`self.K2_SetActorLocation` _presenttower (`KismetMathLibrary.MakeVector` (.x (.location _instancetransform)) (.y (.location _instancetransform)) (+ (.z (.location _instancetransform)) (/ (* (`/Game/BluePrints/GamePlay/TileManager.SizeOfTile` _astile_manager) (`/Game/BluePrints/GamePlay/TileManager.SizeOfMesh` _astile_manager)) 2.0))) false false))
            (:`CastFailed`
              (`self.K2_SetActorLocation` _presenttower _location false false))))))
    (:`then_1`
      (`self.K2_SetActorRotation` (`KismetMathLibrary.MakeRotator` _returnvalue_roll (`KismetMathLibrary.FClamp` _returnvalue_pitch -20.0 60.0) _returnvalue_yaw)))))

(event `InputAction|ZoomOut`
  (params (Key :type "Key Structure"))
  ;[1 1 1] CameraControl
  (:`Pressed`
    (`self.K2_AddActorWorldRotation` self (`KismetMathLibrary.MakeRotator` 0.0 (* (`self.RotateSpeed`) 1.0)) false false)))

(event `InputAction|Confirem`
  (params (Key :type "Key Structure"))
  (bind _presenttower (`self.PresentTower`))
  (bind (_bblockinghit _binitialoverlap _time _distance _location _impactpoint _normal _impactnormal _physmat _hitactor) (`GameplayStatics.BreakHitResult` (`self.HitInfo`)))
  ;[1 1 1] ConfirmBuild
  (:`Pressed`
    (bind _asbp_tdplayercontroller (cast `/Game/BluePrints/GamePlay/BP_TDPlayercontroller` (`GameplayStatics.GetPlayerController` 0)))
    (`/Engine/EditorBlueprintResources/StandardMacros.IsValid` _presenttower
      (:`Is Valid`
        (bind _astile_manager (cast `/Game/BluePrints/GamePlay/TileManager` _hitactor))
        (bind _instancetransform (`/Game/BluePrints/GamePlay/TileManager.GetInstanceTransform` _astile_manager _location))
        (`/Game/BluePrints/GamePlay/BP_TDPlayercontroller.ConfirmBuild` _asbp_tdplayercontroller _presenttower (`KismetMathLibrary.MakeVector` (.x (.location _instancetransform)) (.y (.location _instancetransform)) (+ (.z (.location _instancetransform)) (/ (* (`/Game/BluePrints/GamePlay/TileManager.SizeOfTile` _astile_manager) (`/Game/BluePrints/GamePlay/TileManager.SizeOfMesh` _astile_manager)) 2.0))) _astile_manager)))))

(fn `UserConstructionScript`
  (set `SpringArmComponent.TargetArmLength` (`self.ArmLength`) (`self.SpringArm`)))