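; Tower defense game mode that drives enemy waves and handles the save game.
; BeginPlay finds the spawner manager for the wave count, then loads the "TDSave" slot or creates a new save object.
; WaveEvent triggers the next wave on the manager and records its number; GameSaving stores the player camera's money, clears IsLoad and writes the slot.
; Loading only prints status: restoring towers, wave and money is unfinished, with tower-spawn nodes left unconnected.
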(event `self.ReceiveBeginPlay`
  (`|ExecutionSequence`
    (:`then_0`
      (set `self.IndexOfWave` 0)
      (bind _outactors (`GameplayStatics.GetAllActorsOfClass` "/Game/BluePrints/Enemy/EnenmySpawner/BP_EnemySpawnerManager.BP_EnemySpawnerManager_C"))
      (bind _output_get (set `self.EnemySpawnManager` (`|GetArrayItem` _outactors)))
      (set `self.WaveCount` (- (`KismetArrayLibrary.Array_Length` (`/Game/BluePrints/Enemy/EnenmySpawner/BP_EnemySpawnerManager.WaveManager` _output_get)) 1)))
    (:`then_1`
      (bind _returnvalue (`GameplayStatics.LoadGameFromSlot` "TDSave"))
      (`/Engine/EditorBlueprintResources/StandardMacros.IsValid` _returnvalue
        (:`Is Valid`
          (bind _asmy_save_game (cast `/Game/BluePrints/GamePlay/GameSaving/MySaveGame` _returnvalue))
          (bind _output_get_2 (set `self.SaveGameInstance` _asmy_save_game))
          (if (`/Game/BluePrints/GamePlay/GameSaving/MySaveGame.IsLoad?` _output_get_2)
            (`KismetSystemLibrary.PrintString` "Loading")
            (`KismetSystemLibrary.PrintString` (`KismetStringLibrary.Conv_IntToString` (`KismetArrayLibrary.Array_Length` (`/Game/BluePrints/GamePlay/GameSaving/MySaveGame.TowerMessages` (`self.SaveGameInstance`)))))
            (else
              (`KismetSystemLibrary.PrintString` "NewGame"))))
        (:`Is Not Valid`
          (bind _returnvalue_2 (`GameplayStatics.CreateSaveGameObject` "/Game/BluePrints/GamePlay/GameSaving/MySaveGame.MySaveGame_C"))
          (set `self.SaveGameInstance` _returnvalue_2))))))

(event `WaveEvent`
  ;[1 1 1] NextWave
  (if (<= (`self.IndexOfWave`) (`self.WaveCount`))
    (`/Game/BluePrints/Enemy/EnenmySpawner/BP_EnemySpawnerManager.EachWaveEvent` (`self.EnemySpawnManager`) (`self.IndexOfWave`))
    (bind _result (`/Engine/EditorBlueprintResources/StandardMacros.IncrementInt` (`self.IndexOfWave`))
      (:`  `
        (set `/Game/BluePrints/GamePlay/GameSaving/MySaveGame.WaveNum` _result (`self.SaveGameInstance`))))))

(event `GameSaving`
  (bind _savegameinstance (`self.SaveGameInstance`))
  (set `/Game/BluePrints/GamePlay/GameSaving/MySaveGame.LeftMoney` (`/Game/BluePrints/GamePlay/BP_CameraPawn.LeftMoney` (`/Game/BluePrints/GamePlay/BP_TDPlayercontroller.PlayerCamera` (cast `/Game/BluePrints/GamePlay/BP_TDPlayercontroller` (`GameplayStatics.GetPlayerController` 0) :!pure true))) _savegameinstance)
  (set `/Game/BluePrints/GamePlay/GameSaving/MySaveGame.IsLoad?` false _savegameinstance)
  (`GameplayStatics.SaveGameToSlot` _savegameinstance (`/Game/BluePrints/GamePlay/GameSaving/MySaveGame.SaveSlotName` _savegameinstance) (`/Game/BluePrints/GamePlay/GameSaving/MySaveGame.UserIndex` _savegameinstance))
  (`KismetSystemLibrary.PrintString` "Save done."))

(fn `UserConstructionScript`)