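; BP_BuildingArea is a placement marker actor for building areas, showing whether a building is on it.
; On BeginPlay it creates a dynamic material from M_BaseColor on its cube, lowers the "O" parameter and hides itself.
; Invisible and Visble events toggle its visibility.
; Every Tick it tints the cube green when IsBuildingOnIt is set and grey otherwise.
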(event `self.ReceiveBeginPlay`
  (bind _returnvalue (`PrimitiveComponent.CreateDynamicMaterialInstance` (`self.Cube`) 0 "/Game/Assets/M_BaseColor.M_BaseColor" "None"))
  (bind _output_get (set `self.MaterialInstance` _returnvalue))
  (`MaterialInstanceDynamic.SetScalarParameterValue` _output_get "O" 0.2)
  (`self.Invisible`))

(event `Invisible`
  (`self.SetActorHiddenInGame` self true))

(event `Visble`
  (`self.SetActorHiddenInGame` self false))

(event `self.ReceiveTick`
  (params (DeltaSeconds :type "Float (single-precision)"))
  (if (`self.IsBuildingOnIt`)
    (`MaterialInstanceDynamic.SetVectorParameterValue` (`self.MaterialInstance`) "BaseColor" (struct :`R` 0.010323 :`G` 1.0 :`A` 1.0))
    (else
      (`MaterialInstanceDynamic.SetVectorParameterValue` (`self.MaterialInstance`) "BaseColor" (struct :`R` 0.348958 :`G` 0.348958 :`B` 0.348958 :`A` 1.0)))))

(fn `UserConstructionScript`)