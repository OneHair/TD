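; Player controller for a tower defense game that handles pausing, main HUD creation and tower placement.
; It caches the camera pawn, which holds the pending tower and remaining money.
; A temporary tower spawns with firing disabled and is destroyed on cancel if awaiting confirmation.
; Confirming on a free tile instance marks it occupied, moves and arms the tower, and deducts its cost.
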(event `InputAction|PauseGame`
  (params (Key :type "Key Structure"))
  ;[1 1 1] PauseGame
  (:`Pressed`
    (`GameplayStatics.SetGamePaused` true)
    (bind _returnvalue (`|CreateWidget` "/Game/UMG/PauseMenu.PauseMenu_C"))
    (`UserWidget.AddToViewport` _returnvalue 0)))

(event `self.ReceiveBeginPlay`
  ;[1 1 1] Initial
  (bind _asbp_camera_pawn (cast `/Game/BluePrints/GamePlay/BP_CameraPawn` (`self.K2_GetPawn`)))
  (set `self.PlayerCamera` _asbp_camera_pawn)
  (bind _returnvalue (`|CreateWidget` "/Game/UMG/MainButton.MainButton_C"))
  (`UserWidget.AddToViewport` _returnvalue 0))

(event `CreateTempTower`
  (params (TowerClass :type "/Game/BluePrints/Tower/BP_TowerBase Class Reference"))
  ;[1 1 1] Create tower which doesnt finish building
  (bind _returnvalue (`|SpawnActorFromClass` TowerClass (`KismetMathLibrary.MakeTransform` (0.0 0.0 0.0)) "AlwaysSpawn" "OverrideRootScale" null 100.0 (struct) null))
  (bind _output_get (set `/Game/BluePrints/GamePlay/BP_CameraPawn.PresentTower` _returnvalue (`self.PlayerCamera`)))
  (set `/Game/BluePrints/Tower/BP_TowerBase.CanFire?` false _output_get))

(event `InputAction|Cancel`
  (params (Key :type "Key Structure"))
  (bind _playercamera (`self.PlayerCamera`))
  (bind _presenttower (`/Game/BluePrints/GamePlay/BP_CameraPawn.PresentTower` _playercamera))
  ;[1 1 1] CancelBuild
  (:`Pressed`
    (if (`self.ReadyToConfirm`)
      (set `self.ReadyToConfirm` false)
      (`/Engine/EditorBlueprintResources/StandardMacros.IsValid` _presenttower
        (:`Is Valid`
          (`self.K2_DestroyActor` _presenttower)
          (set `/Game/BluePrints/GamePlay/BP_CameraPawn.PresentTower` null _playercamera))))))

(event `ConfirmBuild`
  (params (PresentTower :type "/Game/BluePrints/Tower/BP_TowerBase Object Reference") (BuildingLocation :type "Vector Structure") (PresentTile :type "/Game/BluePrints/GamePlay/TileManager Object Reference"))
  (bind _hasbuilding (`/Game/BluePrints/GamePlay/TileManager.HasBuilding` PresentTile))
  (bind _playercamera (`self.PlayerCamera`))
  (bind _index (`/Game/BluePrints/GamePlay/TileManager.GetInstanceIndex` PresentTile BuildingLocation))
  (if (not (`|GetArrayItem` _hasbuilding _index))
    (`KismetArrayLibrary.Array_Set` _hasbuilding _index true)
    (`self.K2_SetActorLocation` PresentTower BuildingLocation false false)
    (set `/Game/BluePrints/Tower/BP_TowerBase.CanFire?` true PresentTower)
    ;[1 1 1] MoneyCost
    (set `/Game/BluePrints/GamePlay/BP_CameraPawn.LeftMoney` (- (`/Game/BluePrints/GamePlay/BP_CameraPawn.LeftMoney` _playercamera) (`/Game/BluePrints/Tower/BP_TowerBase.Cost` PresentTower)) _playercamera)
    (set `/Game/BluePrints/GamePlay/BP_CameraPawn.PresentTower` null (`self.PlayerCamera`))
    (set `self.ReadyToConfirm` false)))

(fn `UserConstructionScript`)