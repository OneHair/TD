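; TileManager is a grid actor that lays out tiles as mesh instances and tracks which ones hold buildings.
; The construction script fills a TileX by TileY grid of Tile instances.
; GetInstanceIndex and GetInstanceTransform map a world location to the nearest tile by clamping and rounding its offset from the actor.
; BeginPlay builds the per-tile HasBuilding array and flags the tiles under valid towers in TowerArray.
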(event `self.ReceiveBeginPlay`
  ;[1 1 1] Initialization
  (for _ (range (`InstancedStaticMeshComponent.GetInstanceCount` (`self.Tile`)))
    (`KismetArrayLibrary.Array_Add` (`self.HasBuilding`))
    (for _array_element (`self.TowerArray`)
      (`/Engine/EditorBlueprintResources/StandardMacros.IsValid` _array_element
        (:`Is Valid`
          (bind _index (`self.GetInstanceIndex` (`self.K2_GetActorLocation` _array_element)))
          (`KismetArrayLibrary.Array_Set` (`self.HasBuilding`) _index true))))))

(fn `GetInstanceIndex`
  (params (TargetActorLoaction :type "Vector Structure"))
  (returns (Index :type Integer))
  (bind (_returnvalue_x _returnvalue_y) (`KismetMathLibrary.BreakVector` (- TargetActorLoaction (`self.K2_GetActorLocation`))))
  (bind _returnvalue (* (`self.SizeOfMesh`) (`self.SizeOfTile`)))
  (bind _returnvalue_2 (/ _returnvalue 2.0))
  (bind _returnvalue_3 (`KismetMathLibrary.FClamp` _returnvalue_y 0.0 (* _returnvalue (`KismetMathLibrary.Conv_IntToDouble` (`self.Tile_Y`)))))
  (bind _returnvalue_4 (`KismetMathLibrary.FClamp` _returnvalue_x 0.0 (* _returnvalue (`KismetMathLibrary.Conv_IntToDouble` (`self.Tile_X`)))))
  (bind _returnvalue_5 (`KismetMathLibrary.FTrunc` (/ _returnvalue_3 _returnvalue)))
  (bind _returnvalue_6 (`KismetMathLibrary.FTrunc` (/ _returnvalue_4 _returnvalue)))
  (set `self.Index_X_TEMP` 0)
  (set `self.Index_Y_TEMP` 0)
  (if (< (mod _returnvalue_4 _returnvalue) _returnvalue_2)
    (set `self.Index_X_TEMP` _returnvalue_6)
    (else
      (set `self.Index_X_TEMP` (+ _returnvalue_6 1))))
  (if (< (mod _returnvalue_3 _returnvalue) _returnvalue_2)
    (set `self.Index_Y_TEMP` _returnvalue_5)
    (else
      (set `self.Index_Y_TEMP` (+ _returnvalue_5 1))))
  (return (+ (* (`self.Index_Y_TEMP`) (`self.Tile_X`)) (`self.Index_X_TEMP`))))

(fn `GetInstanceTransform`
  (params (TargetAtorLoaction :type "Vector Structure"))
  (returns (InstanceTransform :type "Transform Structure"))
  (bind (_returnvalue_x _returnvalue_y) (`KismetMathLibrary.BreakVector` (- TargetAtorLoaction (`self.K2_GetActorLocation`))))
  (bind _returnvalue (* (`self.SizeOfMesh`) (`self.SizeOfTile`)))
  (bind _returnvalue_2 (/ _returnvalue 2.0))
  (bind _returnvalue_3 (`KismetMathLibrary.FClamp` _returnvalue_y 0.0 (* _returnvalue (`KismetMathLibrary.Conv_IntToDouble` (`self.Tile_Y`)))))
  (bind _returnvalue_4 (`KismetMathLibrary.FClamp` _returnvalue_x 0.0 (* _returnvalue (`KismetMathLibrary.Conv_IntToDouble` (`self.Tile_X`)))))
  (bind _returnvalue_5 (`KismetMathLibrary.FTrunc` (/ _returnvalue_3 _returnvalue)))
  (bind _returnvalue_6 (`KismetMathLibrary.FTrunc` (/ _returnvalue_4 _returnvalue)))
  (set `self.Index_X_TEMP` 0)
  (set `self.Index_Y_TEMP` 0)
  (if (< (mod _returnvalue_4 _returnvalue) _returnvalue_2)
    (set `self.Index_X_TEMP` _returnvalue_6)
    (else
      (set `self.Index_X_TEMP` (+ _returnvalue_6 1))))
  (if (< (mod _returnvalue_3 _returnvalue) _returnvalue_2)
    (set `self.Index_Y_TEMP` _returnvalue_5)
    (else
      (set `self.Index_Y_TEMP` (+ _returnvalue_5 1))))
  (return (`InstancedStaticMeshComponent.GetInstanceTransform` (`self.Tile`) (+ (* (`self.Index_Y_TEMP`) (`self.Tile_X`)) (`self.Index_X_TEMP`)) true)))

(fn `UserConstructionScript`
  (bind _sizeoftile (`self.SizeOfTile`))
  (bind (_returnvalue_x _returnvalue_y _returnvalue_z) (`KismetMathLibrary.BreakVector` (`SceneComponent.K2_GetComponentLocation` (`self.Tile`))))
  (for _index (range 1 (+ (`self.Tile_Y`) 1))
    (for _index_2 (range 1 (+ (`self.Tile_X`) 1))
      (`InstancedStaticMeshComponent.AddInstance` (`self.Tile`) (`KismetMathLibrary.MakeTransform` (`KismetMathLibrary.MakeVector` (+ (* (- _index_2 1) (`self.SizeOfMesh`)) _returnvalue_x) (+ (* (- _index 1) (`self.SizeOfMesh`)) _returnvalue_y) _returnvalue_z) (struct) (`KismetMathLibrary.MakeVector` _sizeoftile _sizeoftile _sizeoftile))))))